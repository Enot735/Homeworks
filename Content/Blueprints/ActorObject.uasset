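; ActorObject is an actor Blueprint with a static mesh that turns continuously.
; A shared RotateActor function combines a given turn with the mesh's world rotation, applying a large offset on BeginPlay and a small fixed step every Tick, independent of delta time.
; The construction script resets the mesh to unit world scale.
; A Click event sets a Color variable, which nothing shown applies to the mesh.
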(event EventBeginPlay
  (CallFunction|RotateActor "0,90.000000, 0"))

(event EventClick
  (Variables|Default|SetColor "0.190000,0.170000,0.190000"))

(event EventTick
  (params (DeltaSeconds :type Float%20%28single-precision%29))
  (CallFunction|RotateActor "0,1.500000,0.000000"))

(fn ConstructionScript
  (Transformation|SetWorldScale3D (Variables|Default|GetStaticMeshComponent) "1.000000,1.000000,1.000000"))

(fn RotateActor
  (params (Turn :type Rotator))
  (Transformation|SetWorldRotation (Variables|Default|GetStaticMeshComponent) (Math|Rotator|CombineRotators (Transformation|GetWorldRotation (Variables|Default|GetStaticMeshComponent)) Turn) false false))